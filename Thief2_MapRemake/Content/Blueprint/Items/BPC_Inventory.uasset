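; Inventory component that stores item data assets with counts and handles the player's selected item.
; Add, remove and switch functions update the item widget, cycling through the map keys and dropping emptied entries.
; UseItem consumes potions, launches physics scouting orbs or charges the bow while held; StopUsingItem fires an arrow with speed scaled by hold time.
; A one-second delay follows potion and arrow use.
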(event `self.ReceiveBeginPlay`
  (bind _keys (`BlueprintMapLibrary.Map_Keys` (`self.AllItems`)))
  (set `self.CurrentItem` (`|GetArrayItem` _keys)))

(event `UseDelay`
  (params (Time :type "Float (double-precision)"))
  (set `self.ItemDelay` true)
  (`KismetSystemLibrary.Delay` Time)
  (set `self.ItemDelay` false))

(fn `AddItem`
  (params (Type :type "/Game/Blueprint/Items/PDA_Item Object Reference") (Number :type Integer :default 1))
  (bind _allitems (`self.AllItems`))
  (bind _allitems_2 (`self.AllItems`))
  (bind (_value _returnvalue) (`BlueprintMapLibrary.Map_Find` _allitems_2 Type))
  (if (`|EnumEquality` "NewEnumerator7" (`/Game/Blueprint/Items/PDA_Item.Type` Type))
    (`BlueprintMapLibrary.Map_Add` _allitems Type (+ (`BlueprintMapLibrary.Map_Find` _allitems Type) (`/Game/Blueprint/Items/PDA_Item.Value` Type)))
    (elif _returnvalue
      (`BlueprintMapLibrary.Map_Add` _allitems_2 Type (+ _value Number))
      (else
        (`BlueprintMapLibrary.Map_Add` _allitems_2 Type Number))))
  (`/Game/Blueprint/GUI/WBP_Item.UpdateItemAmount` (`self.ItemWidget`)))

(fn `RemoveItem`
  (params (Type :type "/Game/Blueprint/Items/PDA_Item Object Reference") (Amount :type Integer :default 1))
  (returns (Success :type Boolean))
  (bind _allitems (`self.AllItems`))
  (bind (_value _returnvalue) (`BlueprintMapLibrary.Map_Find` _allitems Type))
  (if (`|EnumEquality` (`/Game/Blueprint/Items/PDA_Item.Type` Type) "NewEnumerator3")
    (return false)
    (elif _returnvalue
      (if (> Amount _value)
        (return false)
        (else
          (`BlueprintMapLibrary.Map_Add` _allitems Type (- _value Amount))
          (if (== (`BlueprintMapLibrary.Map_Find` (`self.AllItems`) (`local.Type`)) 0)
            (`self.SwitchItem` false)
            (`BlueprintMapLibrary.Map_Remove` (`self.AllItems`) (`local.Type`))
            (else
              (`/Game/Blueprint/GUI/WBP_Item.UpdateItemAmount` (`self.ItemWidget`))))
          (return true))))))

(fn `StopUsingItem`
  (locals (TypeArrow :type "/Game/Blueprint/Items/Arrows/E_ArrowType Enum" :default "NewEnumerator0"))
  (bind _returnvalue (`self.GetOwner`))
  (bind _currentitem (`self.CurrentItem`))
  (bind (_returnvalue_location _returnvalue_rotation) (`KismetMathLibrary.BreakTransform` (`Actor.GetTransform` _returnvalue)))
  (bind _returnvalue_2 (`Controller.GetControlRotation` (`GameplayStatics.GetPlayerController` 0)))
  (if (not (`self.ItemDelay`))
    (switch `/Game/Blueprint/Items/E_ItemType` (`/Game/Blueprint/Items/PDA_Item.Type` (`self.CurrentItem`))
      (:`NewEnumerator6`
        ;[1 1 1 1 50] Arrows
        (if (>= (`self.HoldTimer`) 0.5)
          (set `local.TypeArrow` (`/Game/Blueprint/Items/PDA_Item.ArrowType` _currentitem))
          (`self.RemoveItem` _currentitem)
          (bind _asbp_player_character (cast `/Game/Blueprint/Character/BP_PlayerCharacter` _returnvalue)
            (:`then`
              (`|SpawnActorFromClass` "/Game/Blueprint/Items/Arrows/BP_Arrow.BP_Arrow_C" (`KismetMathLibrary.MakeTransform` (+ (`SceneComponent.K2_GetComponentLocation` (`/Game/Blueprint/Character/BP_PlayerCharacter.Camera` _asbp_player_character)) (* (`KismetMathLibrary.GetForwardVector` _returnvalue_2) 100.0) (0.0 0.0 -10.0)) _returnvalue_2) "Undefined" "MultiplyWithRoot" null (* (- (`self.HoldTimer`) 0.3) 70.0) (`local.TypeArrow`) _returnvalue null)
              (`/Game/Blueprint/Character/BP_PlayerCharacter.ShowBow` _asbp_player_character false))
            (:`CastFailed`
              (`|SpawnActorFromClass` "/Game/Blueprint/Items/Arrows/BP_Arrow.BP_Arrow_C" (`KismetMathLibrary.MakeTransform` (+ _returnvalue_location (* (`Actor.GetActorForwardVector` _returnvalue) 60.0)) _returnvalue_rotation) "Undefined" "MultiplyWithRoot" null (* (- (`self.HoldTimer`) 0.3) 70.0) (`local.TypeArrow`) _returnvalue null)))
          (set `self.HoldTimer` 0.0)
          (`self.UseDelay` 1.0)
          (else
            (set `self.HoldTimer` 0.0)
            (bind _asbp_player_character_2 (cast `/Game/Blueprint/Character/BP_PlayerCharacter` _returnvalue))
            (`/Game/Blueprint/Character/BP_PlayerCharacter.ShowBow` _asbp_player_character_2 false)))))))

(fn `SwitchItem`
  (params (Right :type Boolean))
  (bind _keys (`BlueprintMapLibrary.Map_Keys` (`self.AllItems`)))
  (if Right
    (bind _returnvalue (`KismetArrayLibrary.Array_Find` _keys (`self.CurrentItem`)))
    (bind _returnvalue_2 (`KismetArrayLibrary.Array_Length` _keys))
    (set `self.CurrentItem` (`|GetArrayItem` _keys (mod (+ _returnvalue 1) _returnvalue_2)))
    (else
      (bind _returnvalue_3 (- _returnvalue 1))
      (set `self.CurrentItem` (`|GetArrayItem` _keys (`KismetMathLibrary.SelectInt` _returnvalue_3 (- _returnvalue_2 1) (>= _returnvalue_3 0))))))
  (`/Game/Blueprint/GUI/WBP_Item.ChangeItem` (`self.ItemWidget`) (`self.CurrentItem`)))

(fn `UseItem`
  (bind _currentitem (`self.CurrentItem`))
  (if (not (`self.ItemDelay`))
    (switch `/Game/Blueprint/Items/E_ItemType` (`/Game/Blueprint/Items/PDA_Item.Type` _currentitem)
      (:`NewEnumerator2`
        (bind _success (`self.RemoveItem` _currentitem))
        (if _success
          (`self.UseDelay` 1.0)))
      (:`NewEnumerator6`
        (bind _asbp_player_character (cast `/Game/Blueprint/Character/BP_PlayerCharacter` (`self.GetOwner`))
          (:`then`
            (`/Game/Blueprint/Character/BP_PlayerCharacter.ShowBow` _asbp_player_character true)
            (`/Game/Blueprint/Character/BP_PlayerCharacter.MoveArrow` _asbp_player_character (`self.HoldTimer`)))
          (:`CastFailed`
            _))
        (set `self.HoldTimer` (`KismetMathLibrary.FClamp` (+ (`GameplayStatics.GetWorldDeltaSeconds`) (`self.HoldTimer`)) 0.0 1.5)))
      (:`NewEnumerator8`
        (`self.RemoveItem` "/Game/Blueprint/Items/DA_ScoutingOrb.DA_ScoutingOrb")
        (bind _asbp_player_character_2 (cast `/Game/Blueprint/Character/BP_PlayerCharacter` (`self.GetOwner`)))
        (bind _muzzle (`/Game/Blueprint/Character/BP_PlayerCharacter.Muzzle` _asbp_player_character_2))
        (bind _returnvalue (`|SpawnActorFromClass` "/Game/Blueprint/ScoutingOrb/BP_ScoutingOrb.BP_ScoutingOrb_C" (`SceneComponent.K2_GetComponentToWorld` _muzzle) "Undefined" "MultiplyWithRoot" null null))
        (bind _sphere (`/Game/Blueprint/ScoutingOrb/BP_ScoutingOrb.Sphere` _returnvalue))
        (`PrimitiveComponent.SetSimulatePhysics` _sphere true)
        (`PrimitiveComponent.AddImpulse` _sphere (* (`SceneComponent.GetForwardVector` _muzzle) 50000.0) "None" false)))))