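; Player ability component for the Scarabée, handling both deployment and recall through UseCapacity.
; When usable, it sphere-traces from the player camera and, if clear, spawns BP_Scarabée at the trace end with camera yaw, then disables further spawning.
; The offset multiplies camera forward by an X-only vector, so it follows only world X.
; Later uses tell the existing scarab to rewind to the player by checkpoint.
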(event `/Game/Blueprint/Scarabée/BPI_Capacity.Use Capacity`
  (bind `_scarabé` (`self.Scarabé`))
  (bind _camera (`/Game/Blueprint/Character/BP_PlayerCharacter.Camera` (cast `/Game/Blueprint/Character/BP_PlayerCharacter` (`GameplayStatics.GetPlayerCharacter` 0) :!pure true)))
  (bind _returnvalue (`SceneComponent.K2_GetComponentLocation` _camera))
  (bind _returnvalue_2 (+ _returnvalue (* (`SceneComponent.GetForwardVector` _camera) (250.0 0.0 0.0))))
  (if (`self.CanBeUsed?`)
    (bind (_outhit _returnvalue_3) (`KismetSystemLibrary.SphereTraceSingle` _returnvalue _returnvalue_2 5.0 "TraceTypeQuery1"))
    (if (not _returnvalue_3)
      (bind _returnvalue_4 (`|SpawnActorFromClass` "/Game/Blueprint/Scarabée/BP_Scarabée.BP_Scarabée_C" (`KismetMathLibrary.MakeTransform` _returnvalue_2 (`KismetMathLibrary.MakeRotator` 0.0 0.0 (.yaw (`SceneComponent.K2_GetComponentRotation` _camera)))) "AlwaysSpawn" "MultiplyWithRoot" null null))
      (set `self.Scarabé` _returnvalue_4)
      (set `self.CanBeUsed?` false))
    (else
      (`/Engine/EditorBlueprintResources/StandardMacros.IsValid` `_scarabé`
        (:`Is Valid`
          (`/Game/Blueprint/Scarabée/BP_Scarabée.RewindToPlayerByCheckPoint` `_scarabé`))))))