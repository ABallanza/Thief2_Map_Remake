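; BP_IAGuard is a guard enemy character that walks forward along the world X axis in repeated steps.
; On BeginPlay it adds itself to the enemy references array in BP_GameMode, then starts Move.
; Move uses AIC_Enemy with AIMoveTo toward a fixed offset from the current location, then calls itself after a short delay when the move finishes.
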(event `self.ReceiveBeginPlay`
  ;[1 1 1] Event Begin Play
  ;;[0.09896 0.09896 0.09896] Récupère la ref au Game Mode et lui en envoie la sienne
  (bind _asbp_game_mode (cast `/Game/Blueprint/BP_GameMode` (`GameplayStatics.GetGameMode`)))
  (bind _output_get (set `self.Game Mode Ref` _asbp_game_mode))
  (`KismetArrayLibrary.Array_Add` (`/Game/Blueprint/BP_GameMode.Enemy References Array` _output_get) self)
  (`self.Move`))

(event `self.ReceiveTick`
  (params (DeltaSeconds :type "Float (single-precision)")))

(event `Move`
  (bind _asaic_enemy (cast `/Game/Blueprint/Enemis/Guard/AIC_Enemy` (`self.GetController`)))
  (`AITask_MoveTo.AIMoveTo` _asaic_enemy (+ (`self.K2_GetActorLocation`) (500.0 0.0 0.0)) null
    (:`OnMoveFinished`
      (`KismetSystemLibrary.Delay` 2.0)
      (`self.Move`))))

(fn `UserConstructionScript`)