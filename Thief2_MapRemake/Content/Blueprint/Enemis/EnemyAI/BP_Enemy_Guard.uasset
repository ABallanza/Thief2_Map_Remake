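; Guard enemy Blueprint that can carry a key in its pocket.
; On BeginPlay it searches ObjectsInPocket for an entry named BP_Key.
; On the first match, it sets the Key child actor component's class to BP_Key and assigns KeyData to the spawned key's ItemDataAsset, then stops searching.
; The construction script only calls its parent.
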(event `self.ReceiveBeginPlay`
  (bind _key (`self.Key`))
  (if (`KismetArrayLibrary.Array_IsNotEmpty` (`self.Objects In Pocket`))
    (for _array_element (`self.Objects In Pocket`)
      (if (`KismetStringLibrary.EqualEqual_StrStr` (`KismetSystemLibrary.GetObjectName` _array_element) "BP_Key")
        (`ChildActorComponent.SetChildActorClass` _key "/Game/Blueprint/Level-Elements/BP_Key.BP_Key_C")
        (bind _asbp_key (cast `/Game/Blueprint/Level-Elements/BP_Key` (`ChildActorComponent.ChildActor` _key)))
        (bind _output_get (set `/Game/Blueprint/Level-Elements/BP_Key.Item Data Asset` (`self.Key Data`) _asbp_key))
        (break)))))

(fn `UserConstructionScript`
  (`parent.UserConstructionScript`))