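; Enemy pawn Blueprint that links itself to its AI controller and sight detection icon and operates doors as it moves.
; A one-time setup on first Tick, rather than BeginPlay, caches AIC_Enemy02 and feeds it to the icon widget.
; Every Tick, forward and closer-point line traces send InteractMessage to any BP_Door hit, throttled by delayed DoOnce resets.
; StartShooting and StopShooting are empty; the rifle trace and damage logic is disconnected.
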(event `self.ReceiveBeginPlay`)

(event `Setuper`
  (bind _asbp_game_mode (cast `/Game/Blueprint/BP_GameMode` (`GameplayStatics.GetGameMode`)))
  (bind _asaic_enemy_02 (cast `/Game/Blueprint/Enemis/EnemyAI/AIC_Enemy02` (`AIBlueprintHelperLibrary.GetAIController` self)))
  (set `self.AIC_REF` _asaic_enemy_02)
  (bind _aswbp_sight_detection_icon (cast `/Game/Blueprint/Enemis/EnemyAI/Widgets/WBP_SightDetectionIcon` (`WidgetComponent.GetUserWidgetObject` (`self.Widget`))))
  (set `/Game/Blueprint/Enemis/EnemyAI/Widgets/WBP_SightDetectionIcon.PawnOwner` self _aswbp_sight_detection_icon)
  (bind _output_get (set `self.SightDetectionIconREF` _aswbp_sight_detection_icon))
  (set `/Game/Blueprint/Enemis/EnemyAI/Widgets/WBP_SightDetectionIcon.AICRef` (`self.AIC_REF`) _output_get))

(event `StartShooting`)

(event `StopShooting`)

(event `self.ReceiveTick`
  (params (DeltaSeconds :type "Float (single-precision)"))
  (bind _returnvalue (`self.K2_GetActorLocation`))
  ;[1 0.8197 0] Event Tick
  (`|ExecutionSequence`
    (:`then_0`
      (`self.Door Opener` _returnvalue (+ _returnvalue (* (`KismetMathLibrary.GetForwardVector` (`self.K2_GetActorRotation`)) 200.0)))
      (`self.DoorCloser` (`KismetMathLibrary.MakeVector` (.x (`self.K2_GetActorLocation`)) (.y (`self.K2_GetActorLocation`)) (+ (.z (`self.K2_GetActorLocation`)) 50.0)) (`SceneComponent.K2_GetComponentLocation` (`self.DoorCloser01`)))
      (`self.DoorCloser` (`self.K2_GetActorLocation`) (`SceneComponent.K2_GetComponentLocation` (`self.DoorCloser02`))))
    (:`then_1`
      (`/Engine/EditorBlueprintResources/StandardMacros.DoOnce` false
        (:`Completed`
          (`self.Setuper`))))))

(event `Door Opener`
  (params (Start :type "Vector Structure") (End :type "Vector Structure"))
  (bind _outhit (`KismetSystemLibrary.LineTraceSingle` Start End "TraceTypeQuery1"))
  (bind (_bblockinghit _binitialoverlap _time _distance _location _impactpoint _normal _impactnormal _physmat _hitactor) (`GameplayStatics.BreakHitResult` _outhit))
  (if (== (`GameplayStatics.GetObjectClass` _hitactor) "/Game/Blueprint/Level-Elements/BP_Door.BP_Door_C")
    (`/Engine/EditorBlueprintResources/StandardMacros.DoOnce` false :!label _label
      (:`Completed`
        (message `/Game/Blueprint/System/Interface/BPI_Interact.Interact` _hitactor null false)
        (`KismetSystemLibrary.Delay` 1.5)
        (goto _label :!via `Reset`)))))

(event `DoorCloser`
  (params (Start :type "Vector Structure") (End :type "Vector Structure"))
  (bind _outhit (`KismetSystemLibrary.LineTraceSingle` Start End "TraceTypeQuery1"))
  (bind (_bblockinghit _binitialoverlap _time _distance _location _impactpoint _normal _impactnormal _physmat _hitactor) (`GameplayStatics.BreakHitResult` _outhit))
  (if (== (`GameplayStatics.GetObjectClass` _hitactor) "/Game/Blueprint/Level-Elements/BP_Door.BP_Door_C")
    (`/Engine/EditorBlueprintResources/StandardMacros.DoOnce` false :!label _label_2
      (:`Completed`
        (message `/Game/Blueprint/System/Interface/BPI_Interact.Interact` _hitactor null false)
        (`KismetSystemLibrary.Delay` 1.5)
        (goto _label_2 :!via `Reset`)))))

(fn `UserConstructionScript`)